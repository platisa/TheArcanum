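; BP_Door is an interactable hinged door that opens only after key flags are collected.
; GetKey events set four key booleans, but Interact checks only Key, Key2 and Key3, leaving Key1 unused.
; When those are set, a FlipFlop alternately plays and reverses DoorTimeline, lerping the mesh yaw to swing it open or closed.
; Box overlap events show and hide a Widget as the interaction prompt.
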(event OnComponentBeginOverlap(Box)
  (params (OverlappedComponent :type Primitive%20Component%20Object%20Reference) (OtherActor :type Actor%20Object%20Reference) (OtherComp :type Primitive%20Component%20Object%20Reference) (OtherBodyIndex :type Integer) (bFromSweep :type Boolean) (SweepResult :type Hit%20Result%20Structure%20%28by%20ref%29))
  ;[1 1 1] Prikazi Mogucnost Interakcije
  (Rendering|SetVisibility (Variables|Default|GetWidget) true false))

(event OnComponentEndOverlap(Box)
  (params (OverlappedComponent :type Primitive%20Component%20Object%20Reference) (OtherActor :type Actor%20Object%20Reference) (OtherComp :type Primitive%20Component%20Object%20Reference) (OtherBodyIndex :type Integer))
  ;[1 1 1] Prikazi Mogucnost Interakcije
  (Rendering|SetVisibility (Variables|Default|GetWidget) false false))

(event EventInteract
  ;[1 1 1] Interakcija - Otvori Zatvori
  (if (Math|Boolean|ANDBoolean (Variables|Default|GetKey?) (Variables|Default|GetKey2?) (Variables|Default|GetKey3?))
    (Utilities|FlowControl|FlipFlop
      (:A
        (bind _door_open (Timeline|Door%20Timeline Play)
          (:Update
            (Transformation|SetRelativeRotation (Variables|Default|GetStaticMesh) (Math|Rotator|MakeRotator 0.0 0.0 (Math|Float|Lerp 0.0 1.1e+02 _door_open)) false false))))
      (:B
        (Timeline|Door%20Timeline Reverse)))))

(event EventGetKey
  ;[1 1 1] Pokupi Kljuc
  (Variables|Default|SetKey? true))

(event EventGetKey1
  ;[1 1 1] Pokupi Kljuc
  (Variables|Default|SetKey1? true))

(event EventGetKey2
  ;[1 1 1] Pokupi Kljuc
  (Variables|Default|SetKey2? true))

(event EventGetKey3
  ;[1 1 1] Pokupi Kljuc
  (Variables|Default|SetKey3? true))

(fn ConstructionScript)